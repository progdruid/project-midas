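; PC_Abyss is a player controller that drives an AbyssPawnBase pawn with free movement and look.
; On BeginPlay it adds the IMC_Abyss Enhanced Input mapping context, and on possess it caches the pawn.
; Input actions forward axis values to the pawn's forward, side and vertical movement functions and its yaw and pitch input.
; Holding X toggles ChangeItemDrag through a raw key binding outside Enhanced Input.
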(event `self.ReceiveBeginPlay`
  (`EnhancedInputSubsystemInterface.AddMappingContext` (pcsubsystem `EnhancedInputLocalPlayerSubsystem` (`GameplayStatics.GetPlayerController` 0)) "/Game/Input/IMC_Abyss.IMC_Abyss" 0 (struct)))

(event `self.ReceivePossess`
  (params (PossessedPawn :type "Pawn Object Reference"))
  (bind _asabyss_pawn_base (cast `AbyssPawnBase` PossessedPawn))
  (set `self.AbyssPawn` _asabyss_pawn_base))

(event `Key|X`
  (params (Key :type "Key Structure"))
  (:`Pressed`
    (`self.ChangeItemDrag` true))
  (:`Released`
    (`self.ChangeItemDrag` false)))

(event `EnhancedInput|/Game/Input/IA_DirectAxis`
  (params (ActionValue :type "Float (double-precision)") (ElapsedSeconds :type "Float (double-precision)") (TriggeredSeconds :type "Float (double-precision)") (InputAction :type "InputAction Object Reference" :default "/Game/Input/IA_DirectAxis.IA_DirectAxis"))
  (:`Triggered`
    (`AbyssPawnBase.MoveForward_Horizontal` (`self.AbyssPawn`) ActionValue)))

(event `EnhancedInput|/Game/Input/IA_SideAxis`
  (params (ActionValue :type "Float (double-precision)") (ElapsedSeconds :type "Float (double-precision)") (TriggeredSeconds :type "Float (double-precision)") (InputAction :type "InputAction Object Reference" :default "/Game/Input/IA_SideAxis.IA_SideAxis"))
  (:`Triggered`
    (`AbyssPawnBase.MoveRight_Horizontal` (`self.AbyssPawn`) ActionValue)))

(event `EnhancedInput|/Game/Input/IA_VerticalAxis`
  (params (ActionValue :type "Float (double-precision)") (ElapsedSeconds :type "Float (double-precision)") (TriggeredSeconds :type "Float (double-precision)") (InputAction :type "InputAction Object Reference" :default "/Game/Input/IA_VerticalAxis.IA_VerticalAxis"))
  (:`Triggered`
    (`AbyssPawnBase.MoveUp_Vertical` (`self.AbyssPawn`) ActionValue)))

(event `EnhancedInput|/Game/Input/IA_Look`
  (params (ActionValue :type "Vector2D Structure") (ElapsedSeconds :type "Float (double-precision)") (TriggeredSeconds :type "Float (double-precision)") (InputAction :type "InputAction Object Reference" :default "/Game/Input/IA_Look.IA_Look"))
  (bind (_x _y) (`KismetMathLibrary.BreakVector2D` ActionValue))
  (bind _abysspawn (`self.AbyssPawn`))
  (:`Triggered`
    (`Pawn.AddControllerYawInput` _abysspawn _x)
    (`Pawn.AddControllerPitchInput` _abysspawn _y)))

(fn `UserConstructionScript`)