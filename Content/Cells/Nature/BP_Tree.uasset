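; A tree cell that spreads by periodically throwing seeds while its surroundings are not too crowded.
; Construction binds handlers to cell start and end, alongside functions that start and stop a looping planting timer.
; Planting spawns a BP_TreeSeed and launches it with a randomized upward impulse angled by MaxSeedAngle.
; A sphere overlap counts nearby trees, pausing the timer above MaxTreesNearToPlant and resuming it otherwise.
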(event `self.Sphere.OnComponentBeginOverlap`
  (params (OverlappedComponent :type "PrimitiveComponent Object Reference") (OtherActor :type "Actor Object Reference") (OtherComp :type "PrimitiveComponent Object Reference") (OtherBodyIndex :type Integer) (bFromSweep :type Boolean) (SweepResult :type "HitResult Structure (by ref)"))
  (cast `/Game/Cells/Nature/BP_Tree` OtherActor)
  (bind _result (`/Engine/EditorBlueprintResources/StandardMacros.IncrementInt` (`self.Trees Near`))
    (:`  `
      (`self.UpdatePlantingByNumTrees` _result))))

(event `self.Sphere.OnComponentEndOverlap`
  (params (OverlappedComponent :type "PrimitiveComponent Object Reference") (OtherActor :type "Actor Object Reference") (OtherComp :type "PrimitiveComponent Object Reference") (OtherBodyIndex :type Integer))
  (cast `/Game/Cells/Nature/BP_Tree` OtherActor)
  (bind _result (`/Engine/EditorBlueprintResources/StandardMacros.DecrementInt` (`self.Trees Near`))
    (:`  `
      (`self.UpdatePlantingByNumTrees` _result))))

(fn `Plant`
  (bind _returnvalue (`KismetMathLibrary.RandomFloatInRange` -360.0 360.0))
  (bind _returnvalue_2 (- 90.0 (`self.Max Seed Angle`)))
  (bind _returnvalue_3 (`KismetMathLibrary.DegCos` _returnvalue_2))
  (bind _returnvalue_4 (`|SpawnActorFromClass` "/Game/Items/BP_TreeSeed.BP_TreeSeed_C" (`SceneComponent.K2_GetComponentToWorld` (`self.Seed Spawn Vector`)) "AdjustIfPossibleButAlwaysSpawn" "MultiplyWithRoot" null null))
  (`/Engine/EditorBlueprintResources/StandardMacros.IsValid` _returnvalue_4
    (:`Is Valid`
      (`PrimitiveComponent.AddImpulse` (`/Game/Items/BP_TreeSeed.Cone` _returnvalue_4) (* (`self.Seed Throw Force`) (`KismetMathLibrary.MakeVector` (* (`KismetMathLibrary.DegSin` _returnvalue) _returnvalue_3) (* (`KismetMathLibrary.DegCos` _returnvalue) _returnvalue_3) (`KismetMathLibrary.DegSin` _returnvalue_2))) "None" true))))

(fn `Start Tree Planting`
  (bind _returnvalue (`KismetSystemLibrary.K2_SetTimerDelegate` (`|CreateDelegate` :!event `Plant`) (`self.Planting Time`) true))
  (set `self.Planting Timer` _returnvalue))

(fn `StopTreePlanting`
  (`KismetSystemLibrary.K2_ClearAndInvalidateTimerHandle` (`self.Planting Timer`)))

(fn `UpdatePlantingByNumTrees`
  (params (`Num Trees Near` :type Integer))
  (bind _planting_timer (`self.Planting Timer`))
  (if (> `Num Trees Near` (`self.Max Trees Near To Plant`))
    (`KismetSystemLibrary.K2_PauseTimerHandle` _planting_timer)
    (else
      (`KismetSystemLibrary.K2_UnPauseTimerHandle` _planting_timer))))

(fn `UserConstructionScript`
  (add `self.OnCellStart` (`|CreateDelegate` :!event `Start Tree Planting`))
  (add `self.OnCellEnd` (`|CreateDelegate` :!event `StopTreePlanting`)))