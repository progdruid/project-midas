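; BP_Gluer is a cell actor that sticks Items to its surface by pulling them along its negative up vector.
; Items entering TriggerBruh are tracked and lose gravity, then regain it on exit.
; Each tick, tracked items receive GlueForce acceleration.
; A second event graph applies StompForce in the same direction to Items currently overlapping the trigger, without toggling gravity.
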(event `self.ReceiveTick`
  (params (DeltaSeconds :type "Float (single-precision)"))
  (for _array_element (`self.Overlapping Items`)
    (`Item.ApplyAcceleration` _array_element (* (`self.GetActorUpVector`) (`self.GlueForce`) -1))))

(event `self.TriggerBruh.OnComponentBeginOverlap`
  (params (OverlappedComponent :type "PrimitiveComponent Object Reference") (OtherActor :type "Actor Object Reference") (OtherComp :type "PrimitiveComponent Object Reference") (OtherBodyIndex :type Integer) (bFromSweep :type Boolean) (SweepResult :type "HitResult Structure (by ref)"))
  (bind _asitem (cast `Item` OtherActor))
  (`KismetArrayLibrary.Array_AddUnique` (`self.Overlapping Items`) _asitem)
  (`Item.ToggleGravity` _asitem false))

(event `self.TriggerBruh.OnComponentEndOverlap`
  (params (OverlappedComponent :type "PrimitiveComponent Object Reference") (OtherActor :type "Actor Object Reference") (OtherComp :type "PrimitiveComponent Object Reference") (OtherBodyIndex :type Integer))
  (bind _asitem (cast `Item` OtherActor))
  (`KismetArrayLibrary.Array_RemoveItem` (`self.Overlapping Items`) _asitem)
  (`Item.ToggleGravity` _asitem true))

(event `self.ReceiveTick`
  (params (DeltaSeconds :type "Float (single-precision)"))
  (for _array_element (`PrimitiveComponent.GetOverlappingActors` (`self.TriggerBruh`) null)
    (bind _asitem (cast `Item` _array_element))
    (`Item.ApplyAcceleration` _asitem (* (`self.GetActorUpVector`) (`self.StompForce`) -1))))

(fn `UserConstructionScript`)

(fn `UserConstructionScript`)