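; BP_Lumberyard is an actor that turns trees entering its overlap sphere into canned air.
; When a BP_Tree overlaps the sphere, ChopTree records the world location of the tree's Cone component and destroys the tree.
; It then spawns a BP_CannedAir at that location, adjusting for collision but always spawning.
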(event `self.Sphere.OnComponentBeginOverlap`
  (params (OverlappedComponent :type "PrimitiveComponent Object Reference") (OtherActor :type "Actor Object Reference") (OtherComp :type "PrimitiveComponent Object Reference") (OtherBodyIndex :type Integer) (bFromSweep :type Boolean) (SweepResult :type "HitResult Structure (by ref)"))
  (bind _asbp_tree (cast `/Game/Cells/Nature/BP_Tree` OtherActor))
  (`/Engine/EditorBlueprintResources/StandardMacros.IsValid` _asbp_tree
    (:`Is Valid`
      (`self.Chop Tree` _asbp_tree))
    (:`Is Not Valid`
      (`KismetSystemLibrary.PrintString` "What"))))

(fn `Chop Tree`
  (params (`Chopped Actor` :type "/Game/Cells/Nature/BP_Tree Object Reference"))
  (bind _output_get (set `self.SavedTreeLocation` (`SceneComponent.K2_GetComponentLocation` (`/Game/Cells/Nature/BP_Tree.Cone` `Chopped Actor`))))
  (`self.K2_DestroyActor` `Chopped Actor`)
  (`|SpawnActorFromClass` "/Game/Items/BP_CannedAir.BP_CannedAir_C" (`KismetMathLibrary.MakeTransform` _output_get) "AdjustIfPossibleButAlwaysSpawn" "MultiplyWithRoot" null null))

(fn `UserConstructionScript`)