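; BP_TreeSeed is a physics-driven seed item that plants a tree where it lands.
; When its Cone component hits a World Static object, it spawns BP_Tree at the hit location, skipping the spawn if no collision-free spot is found, then destroys itself.
; After a one-second grace period from BeginPlay, Tick also destroys the seed once its physics velocity drops to near rest.
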(event `self.ReceiveBeginPlay`
  (`KismetSystemLibrary.Delay` 1.0)
  (set `self.CanSelfDestroy` true))

(event `self.ReceiveTick`
  (params (DeltaSeconds :type "Float (single-precision)"))
  (if (`self.CanSelfDestroy`)
    (bind _returnvalue (`PrimitiveComponent.GetPhysicsLinearVelocity` (`self.Cone`) "None"))
    (if (< (`KismetMathLibrary.VSizeSquared` _returnvalue) 20.0)
      (`self.K2_DestroyActor`))))

(event `self.Cone.OnComponentHit`
  (params (HitComponent :type "PrimitiveComponent Object Reference") (OtherActor :type "Actor Object Reference") (OtherComp :type "PrimitiveComponent Object Reference") (NormalImpulse :type "Vector Structure") (Hit :type "HitResult Structure (by ref)"))
  (`/Engine/EditorBlueprintResources/StandardMacros.IsValid` OtherComp
    (:`Is Valid`
      (switch `ECollisionChannel` (`PrimitiveComponent.GetCollisionObjectType` OtherComp)
        (:`ECC_WorldStatic`
          (`|SpawnActorFromClass` "/Game/Cells/Nature/BP_Tree.BP_Tree_C" (`KismetMathLibrary.Conv_VectorToTransform` (`.Location` (`GameplayStatics.BreakHitResult` Hit))) "AdjustIfPossibleButDontSpawnIfColliding" "MultiplyWithRoot" null null)
          (`self.K2_DestroyActor`))))))

(fn `UserConstructionScript`)